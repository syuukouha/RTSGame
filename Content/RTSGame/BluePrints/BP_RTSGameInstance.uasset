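; Game instance for the RTS game that handles LAN multiplayer sessions through create, find and join events.
; Creating a session opens RTSMap as a listen server.
; Finding sessions searches the LAN for a single result and stores it, and joining uses the first stored entry without checking that one exists.
; Each operation prints its success or failure to screen.
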(event Custom|CreateSession
  (|Session (Game|GetPlayerController 0) 0 true
    (:OnSuccess
      (Game|OpenLevel(byName) "RTSMap" true "?listen")
      (Development|PrintString "CreateSession Success"))
    (:OnFailure
      (Development|PrintString "CreateSession Failure"))))

(event Custom|JoinSession
  (|JoinSession (Game|GetPlayerController 0) (Utilities|Array|Get(acopy) (Variables|Default|GetRef_FindSessionResults))
    (:OnSuccess
      (Development|PrintString "JoinSession Success"))
    (:OnFailure
      (Development|PrintString "JoinSession Failure"))))

(event Custom|FindSessions
  (bind _results (|FindSessions (Game|GetPlayerController 0) 1 true)
    (:OnSuccess
      (bind _output_get (Variables|Default|SetRef_FindSessionResults _results))
      (Development|PrintString (Utilities|String|Append "FindSessions Success.SessionCount:" (Utilities|String|ToString(Integer) (Utilities|Array|Length _output_get)))))
    (:OnFailure
      (Development|PrintString "FindSessions Failure"))))